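; Tactical RPG camera pawn that pans, rotates and zooms around a selected unit.
; Each tick it either snaps to the unit when locked, or matches the unit's height and stays within a maximum horizontal range; manual panning releases the lock.
; Zoom moves a timeline-smoothed point along a perspective spline, deriving spring arm rotation and length from that point and the pivot.
; Yaw rotation is speed-clamped and can be disabled.
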(event `MoveCamera`
  (params (MoveValue :type "Vector2D Structure"))
  (bind (_x _y) (`KismetMathLibrary.BreakVector2D` MoveValue))
  (set `self.bLockCameraToCharacter` false)
  (`self.AddMovementInput` (+ (* (`self.GetActorRightVector`) _x) (* (`self.GetActorForwardVector`) _y)) (`self.MovementSpeed`)))

(event `self.ReceiveTick`
  (params (DeltaSeconds :type "Float (single-precision)"))
  (`self.SelectedUnit`
    (:`then`
      (if (`self.bLockCameraToCharacter`)
        (`self.K2_SetActorLocation` (`self.K2_GetActorLocation` (`self.SelectedUnit`)))
        (elif (> (`KismetMathLibrary.VSizeXY` (- (`self.K2_GetActorLocation`) (`self.K2_GetActorLocation` (`self.SelectedUnit`)))) (`self.MaxCameraRange`))
          (`self.K2_SetActorLocation` (`KismetMathLibrary.MakeVector` (.x (+ (* (`KismetMathLibrary.Normal` (- (`self.K2_GetActorLocation`) (`self.K2_GetActorLocation` (`self.SelectedUnit`)))) (`self.MaxCameraRange`)) (`self.K2_GetActorLocation` (`self.SelectedUnit`)))) (.y (+ (* (`KismetMathLibrary.Normal` (- (`self.K2_GetActorLocation`) (`self.K2_GetActorLocation` (`self.SelectedUnit`)))) (`self.MaxCameraRange`)) (`self.K2_GetActorLocation` (`self.SelectedUnit`)))) (.z (`self.K2_GetActorLocation` (`self.SelectedUnit`)))))
          (else
            (`self.K2_SetActorLocation` (`KismetMathLibrary.MakeVector` (.x (`self.K2_GetActorLocation`)) (.y (`self.K2_GetActorLocation`)) (.z (`self.K2_GetActorLocation` (`self.SelectedUnit`)))))))))
    (:`else`)))

(event `RotateCamera`
  (params (RotateValue :type "Float (double-precision)"))
  (bind (_returnvalue_roll _returnvalue_pitch _returnvalue_yaw) (`KismetMathLibrary.BreakRotator` (`self.K2_GetActorRotation`)))
  (bind _maxrotationspeed (`self.MaxRotationSpeed`))
  (if (`self.bAllowRotation`)
    (`self.K2_SetActorRotation` (`KismetMathLibrary.MakeRotator` _returnvalue_roll _returnvalue_pitch (+ _returnvalue_yaw (`KismetMathLibrary.FClamp` (* RotateValue (`self.RotationSpeed`)) (* _maxrotationspeed -1.0) _maxrotationspeed))))))

(event `ZoomCamera`
  (params (InputValue :type "Float (double-precision)"))
  (bind _output_get (set `self.ZoomPercent` (`KismetMathLibrary.FClamp` (+ (* InputValue (`self.ZoomSpeed`)) (`self.ZoomPercent`)))))
  (`self.SetCameraTransformAlongSpline` _output_get))

(event `SetCameraTransformAlongSpline`
  (params (Time :type "Float (single-precision)"))
  (bind _returnvalue (`SceneComponent.K2_GetComponentLocation` (`self.Pivot`)))
  (set `self.StartSplineTime` (`self.CurrentSplineTime`))
  (bind (_direction _alpha) (`Timeline|Timeline_0` :!via `PlayFromStart`)
    (:`Update`
      (bind _output_get (set `self.CurrentSplineTime` (`KismetMathLibrary.Lerp` (`self.StartSplineTime`) Time _alpha)))
      (bind _returnvalue_2 (`SplineComponent.GetLocationAtTime` (`self.PerspectiveSpline`) _output_get "World" false))
      (`SceneComponent.K2_SetWorldRotation` (`self.SpringArm`) (`KismetMathLibrary.FindLookAtRotation` _returnvalue_2 _returnvalue) false false)
      (set `SpringArmComponent.TargetArmLength` (`KismetMathLibrary.Vector_Distance` _returnvalue _returnvalue_2) (`self.SpringArm`)))))

(fn `AllowCameraRotation`
  (params (bAllow :type Boolean))
  (set `self.bAllowRotation` bAllow))

(fn `Lock Camera To Unit`
  (set `self.bLockCameraToCharacter` true))

(fn `Set Selected Unit`
  (params (Unit :type "/Game/Blueprints/BP_Unit Object Reference"))
  (set `self.SelectedUnit` Unit))

(fn `UserConstructionScript`
  (`self.SetCameraTransformAlongSpline` (`self.ZoomPercent`)))