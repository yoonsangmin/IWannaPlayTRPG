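; Player controller for a turn-based tactical RPG that spawns the party, forwards camera input and runs both exploration and combat turns.
; Outside combat, click-to-move drives the lead unit while companions follow with RVO avoidance.
; In combat, Tick spends each unit's movement budget, clipping long paths, then checks attack range and notifies the game mode.
; Enemy turns also run here, approaching and attacking the player unit with the shortest path.
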(event `CombatDone`
  (set `self.bIsInCombat` false)
  (`|ExecutionSequence`
    (:`then_0`
      (for (_array_element _array_index) (`self.PlayerUnits`)
        (if (!= (`/Game/Blueprints/BP_Unit.HealthPower` _array_element) 0.0)
          (bind _output_get (set `self.CurrentControlUnit` _array_element))
          (set `/Game/Game/BP_TRPGCamera.SelectedUnit` _output_get (`self.CameraActor`))
          (`KismetArrayLibrary.Array_Swap` (`self.PlayerUnits`) 0 _array_index)
          (break))))
    (:`then_1`
      (`self.SetRVO` true)
      (set `/Game/Game/BP_TRPGCamera.bLockCameraToCharacter` true (`self.CameraActor`)))))

(event `self.ReceiveBeginPlay`
  (`EnhancedInputSubsystemInterface.AddMappingContext` (subsystem `EnhancedInputLocalPlayerSubsystem`) "/Game/Input/IMC_TRPG.IMC_TRPG" 0 (struct))
  (bind _returnvalue (`|CreateWidget` "/Game/Widgets/WBP_HUD.WBP_HUD_C"))
  (bind _output_get (set `self.HUD` _returnvalue))
  (`UserWidget.AddToViewport` _output_get 0)
  (bind _returnvalue_2 (`|SpawnActorFromClass` "/Game/Blueprints/BP_Range.BP_Range_C" (`KismetMathLibrary.MakeTransform` (0.0 0.0 0.0)) "Undefined" "MultiplyWithRoot" null null))
  (bind _output_get_2 (set `self.Range` _returnvalue_2))
  (`SceneComponent.SetVisibility` (`Actor.RootComponent` _output_get_2) false true)
  (bind _asbp_trpggame_mode (cast `/Game/Game/BP_TRPGGameMode` (`GameplayStatics.GetGameMode`)))
  (add `/Game/Game/BP_TRPGGameMode.OnPlayerWin` _asbp_trpggame_mode (delegate `CombatDone`)))

(event `EnhancedInput|/Game/Input/InputActions/IA_Select`
  (params (ActionValue :type Boolean) (ElapsedSeconds :type "Float (double-precision)") (TriggeredSeconds :type "Float (double-precision)") (InputAction :type "InputAction Object Reference" :default "/Game/Input/InputActions/IA_Select.IA_Select"))
  (bind (_hitresult _returnvalue) (`self.GetHitResultUnderCursorByChannel` "TraceTypeQuery2"))
  (bind (_hitresult_2 _returnvalue_2) (`self.GetHitResultUnderCursorByChannel` "TraceTypeQuery1"))
  (bind _currentcontrolunit (`self.CurrentControlUnit`))
  (bind _currentcontrolunit_2 (`self.CurrentControlUnit`))
  (bind (_bblockinghit _binitialoverlap _time _distance _location _impactpoint _normal _impactnormal _physmat _hitactor) (`GameplayStatics.BreakHitResult` _hitresult))
  (bind (_bblockinghit_2 _binitialoverlap_2 _time_2 _distance_2 _location_2 _impactpoint_2) (`GameplayStatics.BreakHitResult` _hitresult_2))
  (bind _returnvalue_3 (`self.K2_GetActorLocation` _currentcontrolunit_2))
  (bind (_pathlength _returnvalue_4) (`NavigationSystemV1.GetPathLength` _returnvalue_3 _impactpoint_2 null null))
  (:`Started`
    (if (and (`self.bIsInCombat`) (`self.bIsMovementDone`))
      (if _returnvalue
        (bind _asbp_unit (cast `/Game/Blueprints/BP_Unit` _hitactor))
        (if (`|EnumEquality` (`/Game/Blueprints/BP_Unit.UnitType` _asbp_unit) "NewEnumerator1")
          (if (<= (`self.GetDistanceTo` _asbp_unit _currentcontrolunit) (`/Game/Blueprints/BP_Unit.AttackRange` _currentcontrolunit))
            (`SceneComponent.SetVisibility` (`Actor.RootComponent` (`self.Range`)) false true)
            (`GameplayStatics.ApplyDamage` _hitactor (`/Game/Blueprints/BP_Unit.AttackPower` _currentcontrolunit))
            (bind _asbp_trpggame_mode (cast `/Game/Game/BP_TRPGGameMode` (`GameplayStatics.GetGameMode`)))
            (`/Game/Game/BP_TRPGGameMode.OnAttackDone` _asbp_trpggame_mode))))
      (elif (or (not (`self.bIsInCombat`)) (`self.bIsPlayerTurn`))
        (if _returnvalue_2
          (if (`|EnumEquality` _returnvalue_4 "Success")
            (if (not (`self.bIsInCombat`))
              (`|AIMoveTo` _currentcontrolunit_2 _impactpoint_2 null)
              (elif (< _pathlength (`self.RemainMovementPower`))
                (`|AIMoveTo` (`self.CurrentControlUnit`) _impactpoint_2 null)
                (elif (not (`self.bIsMovementDone`))
                  (bind _returnvalue_5 (`NavigationSystemV1.FindPathToLocationSynchronously` _returnvalue_3 _impactpoint_2 null null))
                  (set `self.PathLength` 0.0)
                  (bind _pathpoints (`NavigationPath.PathPoints` _returnvalue_5))
                  (for _index (range 1 (+ (`KismetArrayLibrary.Array_LastIndex` _pathpoints) 1))
                    (bind _output (`|GetArrayItem` _pathpoints (- _index 1)))
                    (bind _output_2 (`|GetArrayItem` _pathpoints _index))
                    (bind _returnvalue_6 (+ (`self.PathLength`) (`KismetMathLibrary.Vector_Distance` _output _output_2)))
                    (if (> _returnvalue_6 (`self.RemainMovementPower`))
                      (`|AIMoveTo` (`self.CurrentControlUnit`) (+ (* (`KismetMathLibrary.Normal` (- _output_2 _output)) (`KismetMathLibrary.FMax` (- (`self.RemainMovementPower`) (`self.PathLength`)))) _output) null
                        (:`then`
                          (break)))
                      (else
                        (set `self.PathLength` _returnvalue_6)))))))))))))

(event `self.ReceivePossess`
  (params (PossessedPawn :type "Pawn Object Reference"))
  (bind _asbp_trpgcamera (cast `/Game/Game/BP_TRPGCamera` (`self.K2_GetPawn`)))
  (set `self.CameraActor` _asbp_trpgcamera)
  (bind (_success _spawnedunit) (`/Game/Game/BPFL_TRPGFunctionLibrary.SpawnUnit` (`self.GetTransform` (`self.K2_GetPawn`)) "Warrior" "NewEnumerator0" "Player"))
  (if _success
    (`KismetArrayLibrary.Array_Add` (`self.PlayerUnits`) _spawnedunit)
    (bind _output_get (set `self.CurrentControlUnit` _spawnedunit))
    (`/Game/Game/BP_TRPGCamera.Set Selected Unit` (`self.CameraActor`) _output_get)
    ;[1 1 1] 임시로 동료 3명 생성
    (for _ (range 3)
      (bind _randomlocation (`NavigationSystemV1.K2_GetRandomLocationInNavigableRadius` (`self.K2_GetActorLocation` (`self.K2_GetPawn`)) 100.0 null null))
      (bind (_success_2 _spawnedunit_2) (`/Game/Game/BPFL_TRPGFunctionLibrary.SpawnUnit` (`KismetMathLibrary.MakeTransform` _randomlocation) "Wizard" "NewEnumerator0" "Player"))
      (if _success_2
        (`KismetArrayLibrary.Array_Add` (`self.PlayerUnits`) _spawnedunit_2)))
    (`self.SetRVO` true)))

(event `EnhancedInput|/Game/Input/InputActions/IA_MoveCamera`
  (params (ActionValue :type "Vector2D Structure") (ElapsedSeconds :type "Float (double-precision)") (TriggeredSeconds :type "Float (double-precision)") (InputAction :type "InputAction Object Reference" :default "/Game/Input/InputActions/IA_MoveCamera.IA_MoveCamera"))
  (:`Triggered`
    (bind _cameraactor (`self.CameraActor`)
      (:`then`
        (`/Game/Game/BP_TRPGCamera.MoveCamera` _cameraactor ActionValue))
      (:`else`))))

(event `EnhancedInput|/Game/Input/InputActions/IA_NegativeMoveCamera`
  (params (ActionValue :type "Vector2D Structure") (ElapsedSeconds :type "Float (double-precision)") (TriggeredSeconds :type "Float (double-precision)") (InputAction :type "InputAction Object Reference" :default "/Game/Input/InputActions/IA_NegativeMoveCamera.IA_NegativeMoveCamera"))
  (:`Triggered`
    (bind _cameraactor (`self.CameraActor`)
      (:`then`
        (`/Game/Game/BP_TRPGCamera.MoveCamera` _cameraactor ActionValue))
      (:`else`))))

(event `EnhancedInput|/Game/Input/InputActions/IA_LookCameraToCharacter`
  (params (ActionValue :type Boolean) (ElapsedSeconds :type "Float (double-precision)") (TriggeredSeconds :type "Float (double-precision)") (InputAction :type "InputAction Object Reference" :default "/Game/Input/InputActions/IA_LookCameraToCharacter.IA_LookCameraToCharacter"))
  (:`Triggered`
    (bind _cameraactor (`self.CameraActor`)
      (:`then`
        (`/Game/Game/BP_TRPGCamera.Lock Camera To Unit` _cameraactor))
      (:`else`))))

(event `EnhancedInput|/Game/Input/InputActions/IA_RotateCameraGate`
  (params (ActionValue :type Boolean) (ElapsedSeconds :type "Float (double-precision)") (TriggeredSeconds :type "Float (double-precision)") (InputAction :type "InputAction Object Reference" :default "/Game/Input/InputActions/IA_RotateCameraGate.IA_RotateCameraGate"))
  (:`Triggered`
    (bind _cameraactor (`self.CameraActor`)
      (:`then`
        (`/Game/Game/BP_TRPGCamera.AllowCameraRotation` _cameraactor ActionValue))
      (:`else`))))

(event `EnhancedInput|/Game/Input/InputActions/IA_RotateCamera`
  (params (ActionValue :type "Float (double-precision)") (ElapsedSeconds :type "Float (double-precision)") (TriggeredSeconds :type "Float (double-precision)") (InputAction :type "InputAction Object Reference" :default "/Game/Input/InputActions/IA_RotateCamera.IA_RotateCamera"))
  (:`Triggered`
    (bind _cameraactor (`self.CameraActor`)
      (:`then`
        (`/Game/Game/BP_TRPGCamera.RotateCamera` _cameraactor ActionValue))
      (:`else`))))

(event `EnhancedInput|/Game/Input/InputActions/IA_ZoomCamera`
  (params (ActionValue :type "Float (double-precision)") (ElapsedSeconds :type "Float (double-precision)") (TriggeredSeconds :type "Float (double-precision)") (InputAction :type "InputAction Object Reference" :default "/Game/Input/InputActions/IA_ZoomCamera.IA_ZoomCamera"))
  (:`Triggered`
    (bind _cameraactor (`self.CameraActor`)
      (:`then`
        (`/Game/Game/BP_TRPGCamera.ZoomCamera` _cameraactor ActionValue))
      (:`else`))))

(event `self.ReceiveTick`
  (params (DeltaSeconds :type "Float (single-precision)"))
  (bind _playerunits (`self.PlayerUnits`))
  (bind _currentcontrolunit (`self.CurrentControlUnit`))
  (bind _currentcontrolunit_2 (`self.CurrentControlUnit`))
  (bind _currentcontrolunit_3 (`self.CurrentControlUnit`))
  (if (`self.bIsInCombat`)
    (bind _output_get (set `self.RemainMovementPower` (- (`self.RemainMovementPower`) (`KismetMathLibrary.Vector_Distance` (`self.K2_GetActorLocation` (`self.CurrentControlUnit`)) (`self.LastUnitLocation`)))))
    (set `self.LastUnitLocation` (`self.K2_GetActorLocation` (`self.CurrentControlUnit`)))
    (if (< _output_get (`self.MovementEndThreshold`))
      (`/Engine/EditorBlueprintResources/StandardMacros.DoOnce` false :!label _label
        (:`Completed`
          (set `self.bIsMovementDone` true :!label _label_2)
          (`MovementComponent.StopMovementImmediately` (`Character.CharacterMovement` (`self.CurrentControlUnit`)))
          (if (`self.bIsInCombat`)
            (bind _asbp_trpggame_mode (cast `/Game/Game/BP_TRPGGameMode` (`GameplayStatics.GetGameMode`)))
            (`/Game/Game/BP_TRPGGameMode.OnMovementDone` _asbp_trpggame_mode)
            (bind (_outactors _returnvalue) (`KismetSystemLibrary.SphereOverlapActors` (`self.K2_GetActorLocation` _currentcontrolunit_2) (`/Game/Blueprints/BP_Unit.AttackRange` _currentcontrolunit_2) (`|MakeArray` "ObjectTypeQuery3" :!type "EObjectTypeQuery Enum")))
            (set `self.bCanAttack` _returnvalue)
            (for _array_element _outactors
              (if (<= (`self.GetDistanceTo` _array_element _currentcontrolunit) (`/Game/Blueprints/BP_Unit.AttackRange` _currentcontrolunit))
                (bind _asbp_unit (cast `/Game/Blueprints/BP_Unit` _array_element))
                (if (`self.bIsPlayerTurn`)
                  (bind _output_get_2 (set `self.bCanAttack` (`|EnumEquality` (`/Game/Blueprints/BP_Unit.UnitType` _asbp_unit) "NewEnumerator1")))
                  (else
                    (set `self.bCanAttack` (`|EnumEquality` (`/Game/Blueprints/BP_Unit.UnitType` _asbp_unit) "NewEnumerator0"))))
                (if _output_get_2
                  (break))))
            (if (`self.bCanAttack`)
              (`/Game/Blueprints/BP_Range.SetRange` (`self.Range`) (`self.K2_GetActorLocation` _currentcontrolunit_3) (`/Game/Blueprints/BP_Unit.AttackRange` _currentcontrolunit_3))
              (if (not (`self.bIsPlayerTurn`))
                (`KismetSystemLibrary.Delay` 1.0)
                (`SceneComponent.SetVisibility` (`Actor.RootComponent` (`self.Range`)) false true)
                (`GameplayStatics.ApplyDamage` (`self.ShortestPlayer`) (`/Game/Blueprints/BP_Unit.AttackPower` (`self.CurrentControlUnit`)))
                (bind _asbp_trpggame_mode_2 (cast `/Game/Game/BP_TRPGGameMode` (`GameplayStatics.GetGameMode`)))
                (`/Game/Game/BP_TRPGGameMode.OnAttackDone` _asbp_trpggame_mode_2))
              (else
                (bind _asbp_trpggame_mode_3 (cast `/Game/Game/BP_TRPGGameMode` (`GameplayStatics.GetGameMode`)))
                (`/Game/Game/BP_TRPGGameMode.OnAttackDone` _asbp_trpggame_mode_3)))))))
    (else
      (for _index (range 1 (+ (`KismetArrayLibrary.Array_LastIndex` _playerunits) 1))
        (`|AIMoveTo` (`|GetArrayItem` _playerunits _index) (0.0 0.0 0.0) (`|GetArrayItem` _playerunits) 150.0)))))

(event `SetCombatState`
  (params (IsInCombat :type Boolean))
  (set `self.bIsInCombat` IsInCombat)
  (for _array_element (`self.PlayerUnits`)
    (`MovementComponent.StopMovementImmediately` (`Character.CharacterMovement` _array_element)))
  (`self.SetRVO` false))

(event `UpdateCombatState`
  (params (CurrentTurnUnit :type "/Game/Blueprints/BP_Unit Object Reference") (bIsPlayerTurn :type Boolean))
  (bind _playerunits (`self.PlayerUnits`))
  (bind _output (`|GetArrayItem` (`self.PlayerUnits`)))
  (bind _output_get (set `self.CurrentControlUnit` CurrentTurnUnit))
  (set `self.LastUnitLocation` (`self.K2_GetActorLocation` _output_get))
  (set `self.bIsMovementDone` false)
  (bind _output_get_2 (set `self.MaxMovementPower` (`/Game/Blueprints/BP_Unit.MovementPower` (`self.CurrentControlUnit`))))
  (set `self.RemainMovementPower` _output_get_2)
  (bind _cameraactor (`self.CameraActor`)
    (:`then`
      (`/Game/Game/BP_TRPGCamera.Set Selected Unit` _cameraactor (`self.CurrentControlUnit`))
      (`/Game/Game/BP_TRPGCamera.Lock Camera To Unit` _cameraactor)
      (bind _output_get_3 (set `self.bIsPlayerTurn` bIsPlayerTurn))
      (`|ExecutionSequence`
        (:`then_0`
          (goto _label :!via `Reset`))
        (:`then_1`
          (if (not _output_get_3)
            (set `self.ShortestPlayer` _output)
            (set `self.ShortestPathLength` (`NavigationSystemV1.GetPathLength` (`self.K2_GetActorLocation` (`self.CurrentControlUnit`)) (`self.K2_GetActorLocation` _output) null null))
            (for _index (range 1 (+ (`KismetArrayLibrary.Array_LastIndex` _playerunits) 1))
              (bind _output_2 (`|GetArrayItem` _playerunits _index))
              (bind _pathlength (`NavigationSystemV1.GetPathLength` (`self.K2_GetActorLocation` (`self.CurrentControlUnit`)) (`self.K2_GetActorLocation` _output_2) null null))
              (if (< _pathlength (`self.ShortestPathLength`))
                (set `self.ShortestPlayer` _output_2)
                (set `self.ShortestPathLength` _pathlength)))
            (if (<= (`self.ShortestPathLength`) (`/Game/Blueprints/BP_Unit.MovementPower` (`self.CurrentControlUnit`)))
              (`|AIMoveTo` (`self.CurrentControlUnit`) (0.0 0.0 0.0) (`self.ShortestPlayer`) 100.0
                (:`OnSuccess`
                  (goto _label_2)))
              (else
                (bind _returnvalue (`NavigationSystemV1.FindPathToLocationSynchronously` (`self.K2_GetActorLocation` (`self.CurrentControlUnit`)) (`self.K2_GetActorLocation` (`self.ShortestPlayer`)) null null))
                (set `self.PathLength` 0.0)
                (bind _pathpoints (`NavigationPath.PathPoints` _returnvalue))
                (for _index_2 (range 1 (+ (`KismetArrayLibrary.Array_LastIndex` _pathpoints) 1))
                  (bind _output_3 (`|GetArrayItem` _pathpoints (- _index_2 1)))
                  (bind _output_4 (`|GetArrayItem` _pathpoints _index_2))
                  (bind _returnvalue_2 (+ (`self.PathLength`) (`KismetMathLibrary.Vector_Distance` _output_3 _output_4)))
                  (if (> _returnvalue_2 (`self.RemainMovementPower`))
                    (`|AIMoveTo` (`self.CurrentControlUnit`) (+ (* (`KismetMathLibrary.Normal` (- _output_4 _output_3)) (`KismetMathLibrary.FMax` (- (`self.RemainMovementPower`) (`self.PathLength`)))) _output_3) null
                      (:`then`
                        (break)))
                    (else
                      (set `self.PathLength` _returnvalue_2))))))))))
    (:`else`)))

(fn `SetRVO`
  (params (Value :type Boolean))
  (if Value
    (`CharacterMovementComponent.SetAvoidanceEnabled` (`Character.CharacterMovement` (`|GetArrayItem` (`self.PlayerUnits`))) false)
    (for _index (range 1 (+ (`KismetArrayLibrary.Array_LastIndex` (`self.PlayerUnits`)) 1))
      (`CharacterMovementComponent.SetAvoidanceEnabled` (`Character.CharacterMovement` (`|GetArrayItem` (`self.PlayerUnits`) _index)) true))
    (else
      (for _index_2 (range (+ (`KismetArrayLibrary.Array_LastIndex` (`self.PlayerUnits`)) 1))
        (`CharacterMovementComponent.SetAvoidanceEnabled` (`Character.CharacterMovement` (`|GetArrayItem` (`self.PlayerUnits`) _index_2)) false)))))

(fn `UserConstructionScript`)