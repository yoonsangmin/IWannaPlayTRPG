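; BP_Unit is a data-driven unit that takes damage and disappears when its health runs out.
; On BeginPlay it looks up its UnitName row in DT_UnitDataTable, loads the skeletal mesh synchronously and copies the profile image and combat stats.
; AnyDamage spawns a BP_DamageText, clamps health at zero, then hides the unit and disables collision rather than destroying it.
; GetHealthPowerPercent returns current health as a fraction of maximum.
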(event `self.ReceiveBeginPlay`
  (bind _returnvalue (`|GetDataTableRow` "/Game/DataTables/DT_UnitDataTable.DT_UnitDataTable" (`self.UnitName`))
    (:`then`
      (`|ExecutionSequence`
        (:`then_0`
          (bind (_unitmesh _profileimage _unitstats) (break `/Game/DataTables/UnitData` _returnvalue))
          (bind _returnvalue_2 (`KismetSystemLibrary.LoadAsset_Blocking` _unitmesh))
          (bind _asskeletal_mesh (cast `SkeletalMesh` _returnvalue_2))
          (`SkeletalMeshComponent.SetSkeletalMeshAsset` (`self.Mesh`) _asskeletal_mesh))
        (:`then_1`
          (set `self.ProfileImage` _profileimage)
          (bind _output_get (set `self.MaxHealthPower` (break `/Game/DataTables/UnitStats` _unitstats)))
          (set `self.HealthPower` _output_get)
          (set `self.AttackPower` (`.AttackPower_15_1FDC97684A58ACF335A20BA5616BABC4` (break `/Game/DataTables/UnitStats` _unitstats)))
          (set `self.AttackRange` (`.AttackRange_16_8277EC0C45934A47277EC9B6370C9042` (break `/Game/DataTables/UnitStats` _unitstats)))
          (set `self.MovementPower` (`.MovementPower_17_11F0042D4E7E7B476087B4B10F25CECE` (break `/Game/DataTables/UnitStats` _unitstats)))
          (set `self.Dex` (`.Dex_3_8D340A2F4234C85EAF7F2AAE1FCA3AAB` (break `/Game/DataTables/UnitStats` _unitstats))))))))

(event `self.ReceiveAnyDamage`
  (params (Damage :type "Float (single-precision)") (DamageType :type "DamageType Object Reference") (InstigatedBy :type "Controller Object Reference") (DamageCauser :type "Actor Object Reference"))
  (`|SpawnActorFromClass` "/Game/Blueprints/BP_DamageText.BP_DamageText_C" (`self.GetTransform`) "Undefined" "MultiplyWithRoot" null Damage null)
  (bind _output_get (set `self.HealthPower` (`KismetMathLibrary.FMax` (- (`self.HealthPower`) Damage))))
  (if (== _output_get 0.0)
    (`SceneComponent.SetVisibility` (`self.CapsuleComponent`) false true)
    (`PrimitiveComponent.SetCollisionEnabled` (`self.CapsuleComponent`) "NoCollision")
    (`PrimitiveComponent.SetCollisionEnabled` (`self.Mesh`) "NoCollision")))

(fn `GetHealthPowerPercent`
  (returns (HealthPowerPercent :type "Float (double-precision)"))
  (return (/ (`self.HealthPower`) (`self.MaxHealthPower`))))

(fn `UserConstructionScript`)