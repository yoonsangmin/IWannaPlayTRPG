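; BP_EnemyTrigger is a one-shot encounter trigger that starts a TRPG battle when a Player unit overlaps it.
; The construction script fills the Enemies set with Enemy-type BP_Units found by a sphere overlap matching CollisionComp's radius, so the group is captured at construction rather than on overlap.
; On player overlap it passes that set as an array to BP_TRPGGameMode's StartBattle, then destroys itself.
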(event `self.ReceiveActorBeginOverlap`
  (params (OtherActor :type "Actor Object Reference"))
  (bind _asbp_unit (cast `/Game/Blueprints/BP_Unit` OtherActor))
  (switch `/Game/DataTables/EUnitType` (`/Game/Blueprints/BP_Unit.UnitType` _asbp_unit)
    (:`NewEnumerator0`
      (bind _asbp_trpggame_mode (cast `/Game/Game/BP_TRPGGameMode` (`GameplayStatics.GetGameMode`)))
      (bind _result (`BlueprintSetLibrary.Set_ToArray` (`self.Enemies`)))
      (`/Game/Game/BP_TRPGGameMode.StartBattle` _asbp_trpggame_mode _result)
      (`self.K2_DestroyActor`))))

(fn `UserConstructionScript`
  (`BlueprintSetLibrary.Set_Clear` (`self.Enemies`))
  (bind _outactors (`KismetSystemLibrary.SphereOverlapActors` (`self.K2_GetActorLocation`) (`SphereComponent.SphereRadius` (`self.CollisionComp`)) (`|MakeArray` "ObjectTypeQuery3" :!type "EObjectTypeQuery Enum") "/Game/Blueprints/BP_Unit.BP_Unit_C"))
  (for _array_element _outactors
    (bind _asbp_unit (cast `/Game/Blueprints/BP_Unit` _array_element))
    (if (`|EnumEquality` (`/Game/Blueprints/BP_Unit.UnitType` _asbp_unit) "NewEnumerator1")
      (`BlueprintSetLibrary.Set_Add` (`self.Enemies`) _asbp_unit))))